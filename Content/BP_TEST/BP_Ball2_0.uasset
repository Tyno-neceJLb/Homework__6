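; BP_Ball2_0 is a test ball actor that travels in a straight line and bounces off whatever blocks it.
; Tick sweeps a local offset along DirectVector at InitianSpeed, scaled by delta time, and reflects the direction about the surface normal on a blocking hit.
; The Hit event multiplies the speed by ten with a MinSpeed floor, and no upper limit is applied.
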(event Collision|EventActorBeginOverlap
  (params (OtherActor :type Actor%20Object%20Reference)))

(event EventTick
  (params (DeltaSeconds :type Float%20%28single-precision%29))
  (bind _sweephitresult (Transformation|AddActorLocalOffset (* (* (Variables|Default|GetDirectVector) (Variables|Default|Getinitian%20Speed)) DeltaSeconds) true false))
  (if (.bBlockingHit (Collision|BreakHitResult _sweephitresult))
    (Variables|Default|SetDirectVector (Math|Vector|GetReflectionVector (Variables|Default|GetDirectVector) (.Normal (Collision|BreakHitResult _sweephitresult))))))

(event Collision|EventHit
  (params (MyComp :type Primitive%20Component%20Object%20Reference) (Other :type Actor%20Object%20Reference) (OtherComp :type Primitive%20Component%20Object%20Reference) (bSelfMoved :type Boolean) (HitLocation :type Vector :default "0, 0, 0") (HitNormal :type Vector :default "0, 0, 0") (NormalImpulse :type Vector :default "0, 0, 0") (Hit :type Hit%20Result%20Structure%20%28by%20ref%29))
  (Variables|Default|Setinitian%20Speed (Math|Float|Max(Float) (Variables|Default|GetMinSpeed) (* (Variables|Default|Getinitian%20Speed) (Variables|Default|Get-10%25)))))

(fn ConstructionScript)