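; BP_Ball is a test ball actor that moves along a direction vector and bounces by reflection.
; Each tick it makes a swept offset from Direction and Speed, then unconditionally reflects Direction about the sweep's normal, with no blocking-hit check.
; BeginPlay sets the starting Speed.
; Each Hit multiplies Speed tenfold, and a result at or below MinSpeed is clamped and zeroes the sphere's physics velocity.
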(event Collision|EventActorBeginOverlap
  (params (OtherActor :type Actor%20Object%20Reference)))

(event EventTick
  (params (DeltaSeconds :type Float%20%28single-precision%29))
  (bind _sweephitresult (Transformation|AddActorLocalOffset (* (* (Variables|Default|GetDirection) (Variables|Default|GetSpeed)) DeltaSeconds) true false))
  (if true
    (Variables|Default|SetDirection (Math|Vector|GetReflectionVector (Variables|Default|GetDirection) (.Normal (Collision|BreakHitResult _sweephitresult))))))

(event Collision|EventHit
  (params (MyComp :type Primitive%20Component%20Object%20Reference) (Other :type Actor%20Object%20Reference) (OtherComp :type Primitive%20Component%20Object%20Reference) (bSelfMoved :type Boolean) (HitLocation :type Vector :default "0, 0, 0") (HitNormal :type Vector :default "0, 0, 0") (NormalImpulse :type Vector :default "0, 0, 0") (Hit :type Hit%20Result%20Structure%20%28by%20ref%29))
  (Variables|Default|SetSpeed (* (Variables|Default|GetSpeed) (Variables|Default|Get-10%25)))
  (if (<= (Variables|Default|GetSpeed) (Variables|Default|GetMinSpeed))
    (Variables|Default|SetSpeed (Variables|Default|GetMinSpeed))
    (Physics|SetPhysicsLinearVelocity (Variables|Default|GetSphere) "0, 0, 0" false "None")))

(event EventBeginPlay
  (Variables|Default|SetSpeed 1e+01))

(fn ConstructionScript)